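; Game mode for a quick-draw duel between a player swordsman and an NPC, driven by an Intro, Wait, Draw and Finish phase state.
; Tick times the intro, then a random delay leads into Draw, which calls the draw-phase starter and shows the exclamation cue.
; A successful attack defeats the opponent, hides the cue and starts a restart timer.
; Reset restores the intro phase and both swordsmen.
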(event `self.ReceiveBeginPlay`
  (bind _returnvalue (`GameplayStatics.GetActorOfClass` "/Game/Blueprints/BP_Exclamation.BP_Exclamation_C"))
  (set `self.ExcamationRef` _returnvalue)
  (bind _returnvalue_2 (`GameplayStatics.GetActorOfClass` "/Game/Blueprints/BP_SwordsmanPlayer.BP_SwordsmanPlayer_C"))
  (set `self.SwordsmanPlayer` _returnvalue_2)
  (bind _returnvalue_3 (`GameplayStatics.GetActorOfClass` "/Game/Blueprints/BP_SwordsmanNPC.BP_SwordsmanNPC_C"))
  (set `self.SwordsmanNPC` _returnvalue_3))

(event `self.ReceiveTick`
  (params (DeltaSeconds :type "Float (single-precision)"))
  (set `self.ElapsedTime` (+ DeltaSeconds (`self.ElapsedTime`)))
  (switch `/Game/Blueprints/Enums/E_Phase` (`self.Phase`)
    (:`NewEnumerator0`
      (if (>= (`self.ElapsedTime`) (`self.RoundStartTime`))
        (set `self.Phase` "NewEnumerator1")
        (`KismetSystemLibrary.Delay` (`KismetMathLibrary.RandomFloatInRange` (`self.MinDrawDelay`) (`self.MaxDrawDelay`)))
        (set `self.Phase` "NewEnumerator2")
        (`self.DrawPhaseStarter`)
        (`/Engine/EditorBlueprintResources/StandardMacros.IsValid` (`self.ExcamationRef`)
          (:`Is Valid`
            (`/Game/Blueprints/BP_Exclamation.SetVisibility` (`self.ExcamationRef`) true))
          (:`Is Not Valid`
            (`KismetSystemLibrary.PrintString` "Exclamation Not found")))))))

(fn `AttackedSuccesfully`
  (params (IsPlayer :type Boolean))
  (if IsPlayer
    (`/Game/Blueprints/BP_Swordsman.Defeated` (`self.SwordsmanNPC`))
    (else
      (`/Game/Blueprints/BP_Swordsman.Defeated` (`self.SwordsmanPlayer`))))
  (`/Engine/EditorBlueprintResources/StandardMacros.IsValid` (`self.ExcamationRef`)
    (:`Is Valid`
      (`/Game/Blueprints/BP_Exclamation.SetVisibility` (`self.ExcamationRef`) false)
      (`KismetSystemLibrary.K2_SetTimerDelegate` (`|CreateDelegate` :!event `Reset`) (`self.RestardDelay`)))))

(fn `Reset`
  (set `self.Phase` "NewEnumerator0")
  (set `self.ElapsedTime` 0.0)
  (`/Game/Blueprints/BP_Swordsman.Reset` (`self.SwordsmanPlayer`))
  (`/Game/Blueprints/BP_Swordsman.Reset` (`self.SwordsmanNPC`)))

(fn `SetGameFinished`
  (set `self.Phase` "NewEnumerator3"))

(fn `UserConstructionScript`)